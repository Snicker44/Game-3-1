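; BP_Door1 is a locked door that sends the player to LevelTwo when they carry the required key item.
; On BeginPlay it shows the required key on its TextRender.
; When a BP_ThirdPersonCharacter overlaps its Box, it checks that character's Inventory for the key, removes it and opens the level by name.
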(event `self.ReceiveBeginPlay`
  ;[1 1 1] Set the text on the door showing what item is needed
  (`TextRenderComponent.K2_SetText` (`self.TextRender`) (`KismetTextLibrary.Conv_StringToText` (`self.RequeredKey`))))

(event `self.Box.OnComponentBeginOverlap`
  (params (OverlappedComponent :type "PrimitiveComponent Object Reference") (OtherActor :type "Actor Object Reference") (OtherComp :type "PrimitiveComponent Object Reference") (OtherBodyIndex :type Integer) (bFromSweep :type Boolean) (SweepResult :type "HitResult Structure (by ref)"))
  (bind _requeredkey (`self.RequeredKey`))
  ;[1 1 1] Open the door if the player has the right item
  (bind _asbp_third_person_character (cast `/Game/ThirdPerson/Blueprints/BP_ThirdPersonCharacter` OtherActor))
  (if (`KismetArrayLibrary.Array_Contains` (`/Game/ThirdPerson/Blueprints/BP_ThirdPersonCharacter.Inventory` _asbp_third_person_character) _requeredkey)
    (`/Game/ThirdPerson/Blueprints/BP_ThirdPersonCharacter.REmoveItem` _asbp_third_person_character _requeredkey)
    (`GameplayStatics.OpenLevel` "LevelTwo")))

(fn `UserConstructionScript`)